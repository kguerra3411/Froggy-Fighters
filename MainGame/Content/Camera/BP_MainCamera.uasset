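; BP_MainCamera is a shared camera that becomes player 0's view target and follows every actor tagged "Character".
; Each tick it moves smoothly toward their average location and records the farthest one's position.
; The Camera eases back along the Arrow's reversed forward vector by CameraDistance.
; CameraDistanceLogic supplies that distance, though its only visible content is an unconnected clamp calculation based on the farthest character's local offset.
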(event EventBeginPlay
  (Game|Player|SetViewTargetwithBlend (Game|GetPlayerController 0) self 0.0 "VTBlend_Linear" 0.0 false))

(event Collision|EventActorBeginOverlap
  (params (OtherActor :type Actor%20Object%20Reference)))

(event EventTick
  (params (DeltaSeconds :type Float%20%28single-precision%29))
  (Rendering|Debug|FlushPersistentDebugLines)
  (bind _outactors (Actor|GetAllActorswithTag "Character"))
  (Variables|Default|SetMostDistantActor 0.0)
  (for _array_element _outactors
    (if (> (Math|Float|Absolute(Float) (Math|Vector|VectorLength (- (Transformation|GetActorLocation) (Transformation|GetActorLocation _array_element)))) (Variables|Default|GetMostDistantActor))
      (Variables|Default|SetMostDistantActor (Math|Float|Absolute(Float) (Math|Vector|VectorLength (- (Transformation|GetActorLocation) (Transformation|GetActorLocation _array_element)))))
      (Variables|Default|SetMostDistantVector (Transformation|GetActorLocation _array_element))))
  (bind _returnvalue (Class|GameplayStatics|GetActorArrayAverageLocation _outactors))
  (Variables|Default|SetCameraDistance (Utilities|CameraDistanceLogic))
  (CallFunction|SetCameraPosition _returnvalue))

(fn ConstructionScript)

(fn SetCameraPosition
  (params (Target :type Vector))
  (Transformation|SetActorLocation (Math|Interpolation|VInterpTo (Transformation|GetActorLocation) Target (Utilities|Time|GetWorldDeltaSeconds) 5.0) false false)
  (Transformation|SetWorldLocation (Variables|Default|GetCamera) (Math|Interpolation|VInterpTo (Transformation|GetWorldLocation (Variables|Default|GetCamera)) (+ (* (* (Math|Vector|GetForwardVector (Variables|Default|GetArrow)) -1.0) (Variables|Default|GetCameraDistance)) (Transformation|GetActorLocation)) (Utilities|Time|GetWorldDeltaSeconds) 5.0) false false))